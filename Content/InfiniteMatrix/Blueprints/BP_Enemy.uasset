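; BP_Enemy is a short-lived enemy actor that hurts the player on contact and awards score when hit by a projectile.
; It sets a ten-second lifespan on BeginPlay and resolves hits in ActorBeginOverlap by casting the other actor.
; Player overlap decreases health, plays a buzz, destroys the enemy, and flags death and shows restart when health is depleted.
; Projectile overlap increases player zero's score, plays a coin sound and destroys the enemy.
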(event EventBeginPlay
  ;[1 1 1] Despawn
  (Actor|SetLifeSpan 1e+01))

(event Collision|EventActorBeginOverlap
  (params (OtherActor :type Actor%20Object%20Reference))
  (bind _enemymesh (Variables|Default|GetEnemyMesh))
  (bind _returnvalue (Transformation|GetWorldLocation _enemymesh))
  ;[1 1 1] Player and Projectile Collision
  (bind _asbp_player (Utilities|Casting|CastToBP_Player OtherActor)
    (:then
      (Default|DecreaseHealth _asbp_player)
      (Audio|PlaySoundatLocation "/Game/Interface_And_Item_Sounds/WAV/Error_Buzz_01.Error_Buzz_01" _returnvalue "0, 0, 0" 1.0 1.0 0.0 0 0 0 0)
      (Actor|DestroyActor)
      (Math|Float|CompareFloat (Variables|/Game/InfiniteMatrix/Blueprints/BP_Player.BP_Player_C|GetCurrentHealth _asbp_player) 0.0 ; Check if health 0 after decrease and restart
        (:==
          _)
        (:<
          _))
      (Variables|/Game/InfiniteMatrix/Blueprints/BP_Player.BP_Player_C|SetIsDead _asbp_player true)
      (Default|DisplayRestart _asbp_player))
    (:CastFailed
      (Utilities|Casting|CastToBP_Projectile OtherActor)
      (bind _asbp_player_2 (Utilities|Casting|CastToBP_Player (Game|Player|GetPlayerPawn 0)))
      (Default|IncreaseScore _asbp_player_2)
      (Audio|PlaySoundatLocation "/Game/Interface_And_Item_Sounds/Cues/Coins_01_Cue.Coins_01_Cue" _returnvalue "0, 0, 0" 1.0 1.0 0.0 0 0 0 0)
      (Actor|DestroyActor))))

(event EventTick
  (params (DeltaSeconds :type Float%20%28single-precision%29)))

(fn ConstructionScript)